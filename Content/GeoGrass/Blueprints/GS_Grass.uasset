(event Custom|Build
  (bind _last_index (Variables|Default|GetLast%20Index))
  (bind _instancedstaticmesh (Variables|Default|GetInstancedStaticMesh))
  (bind _templayersarray (Variables|Default|GetTempLayersArray))
  (bind _returnvalue (Math|Conversions|ToFloat(Integer) _last_index))
  (for _array_element _templayersarray
    (Components|DestroyComponent _array_element))
  (Utilities|Array|Clear _templayersarray)
  (Utilities|Array|Clear (Variables|Default|GetMaterials))
  (if (Variables|Default|GetPerInstanceData)
    (bind _object (Variables|Default|GetObject)
      (:then
        (Variables|Default|SetOGObject (Variables|/Script/Engine.StaticMeshComponent|GetStaticMesh (Variables|/Script/Engine.StaticMeshActor|GetStaticMeshComponent _object)))
        (Rendering|SetCastShadow _instancedstaticmesh false)
        (Components|Tick|SetComponentTickEnabled _instancedstaticmesh false)
        (bind _output_get (Variables|Default|SetPerInstanceMesh _instancedstaticmesh))
        (bind _returnvalue_2 (Rendering|Material|CreateDynamicMaterialInstance _output_get 0 "/Game/GeoGrass/Materials/Grass/GS_M_Grass.GS_M_Grass" "None" :!class /Script/Engine.PrimitiveComponent))
        (bind _output_get_2 (Variables|Default|SetPerInstanceMaterial _returnvalue_2))
        (Rendering|Material|SetTextureParameterValue _output_get_2 "Grass" (Variables|Default|GetGrassTexture))
        (Rendering|Material|SetScalarParameterValue _output_get_2 "Scale" (Variables|Default|GetUVValue) :!class /Script/Engine.MaterialInstanceDynamic)
        (Rendering|Material|SetScalarParameterValue _output_get_2 "PI" 1.0 :!class /Script/Engine.MaterialInstanceDynamic)
        (for _index (range 1 _last_index)
          (bind _returnvalue_3 (Components|InstancedStaticMesh|AddInstance (Variables|Default|GetPerInstanceMesh) (Math|Transform|MakeTransform (.location (Transformation|GetWorldTransform (Variables|/Script/Engine.StaticMeshActor|GetStaticMeshComponent _object))) (.rotation (Transformation|GetWorldTransform (Variables|/Script/Engine.StaticMeshActor|GetStaticMeshComponent _object))) (.scale (Transformation|GetWorldTransform (Variables|/Script/Engine.StaticMeshActor|GetStaticMeshComponent _object)))) true))
          (Components|StaticMesh|SetStaticMesh (Variables|Default|GetPerInstanceMesh) (Variables|Default|GetOGObject))
          (Components|InstancedStaticMesh|SetCustomDataValue (Variables|Default|GetPerInstanceMesh) _returnvalue_3 1 (Math|Float|Clamp(Float) (Math|Float|MapRangeClamped (Math|Conversions|ToFloat(Integer) _index) 1.0 _returnvalue 0.0 1.0) 0.1 0.99) true)
          (Components|InstancedStaticMesh|SetCustomDataValue (Variables|Default|GetPerInstanceMesh) _returnvalue_3 2 (Math|Float|MapRangeClamped (Math|Float|Power (Math|Float|MapRangeClamped (Math|Conversions|ToFloat(Integer) _index) 1.0 _returnvalue 0.0 1e+01) (Variables|Default|GetExp)) 0.0 (Math|Float|Power (Math|Float|MapRangeClamped _returnvalue 1.0 _returnvalue 0.0 1e+01) (Variables|Default|GetExp)) 0.0 (Variables|Default|GetHeight)) false)))
      (:else
        (Development|PrintString "Please set a Mesh for GS_Grass")))))

(event Custom|CustomEvent_0
  (bind _sphere (Variables|Default|GetSphere))
  (bind _returnvalue (Transformation|GetComponentVelocity _sphere))
  (for _array_element (Variables|Default|GetMaterials)
    (Utilities|IsValid _array_element
      (:Is%20Valid
        (Rendering|Material|SetVectorParameterValue _array_element "vol" (Utilities|Struct|MakeLinearColor (.x _returnvalue) (.y _returnvalue) (.z _returnvalue) 1.0) :!class /Script/Engine.MaterialInstanceDynamic)))))

(event EventTick
  (params (DeltaSeconds :type Float%20%28single-precision%29)))

(event EventBeginPlay
  (CallFunction|Build))

(fn ConstructionScript
  (CallFunction|Build))